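; Interactable button actor that shows and hides an info window (plane, lines and widget) and steps through year states on it.
; Component overlaps trigger the start, plus and less buttons, each faking a press with a short delayed hide or nudge.
; Plus and less move a bounded YearState, update its enum, then push the index to Panel_Widget to change image and year text.
; The year layout switch has no branch logic.
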(event `self.Interactable.OnComponentBeginOverlap`
  (params (OverlappedComponent :type "PrimitiveComponent Object Reference") (OtherActor :type "Actor Object Reference") (OtherComp :type "PrimitiveComponent Object Reference") (OtherBodyIndex :type Integer) (bFromSweep :type Boolean) (SweepResult :type "HitResult Structure (by ref)"))
  (bind _plane (`self.Plane`))
  ;[1 0.2167 0.1869] Start button "animation"
  (`SceneComponent.SetHiddenInGame` (`self.Start_Button`) true false)
  (`KismetSystemLibrary.Delay` 0.4)
  (`SceneComponent.SetHiddenInGame` (`self.Start_Button`) false false)
  (if (`self.isWindowOn`)
    (`SceneComponent.SetHiddenInGame` _plane true false)
    (`SceneComponent.SetHiddenInGame` (`self.Lines`) true false)
    (`SceneComponent.SetHiddenInGame` (`self.UI`) true false)
    (set `self.isWindowOn` false)
    (else
      (`SceneComponent.SetHiddenInGame` _plane false false)
      (`SceneComponent.SetHiddenInGame` (`self.Lines`) false false)
      (`SceneComponent.SetHiddenInGame` (`self.UI`) false false)
      (set `self.isWindowOn` true))))

(event `self.Button_Plus.OnComponentBeginOverlap`
  (params (OverlappedComponent :type "PrimitiveComponent Object Reference") (OtherActor :type "Actor Object Reference") (OtherComp :type "PrimitiveComponent Object Reference") (OtherBodyIndex :type Integer) (bFromSweep :type Boolean) (SweepResult :type "HitResult Structure (by ref)"))
  ;[0.7801 0.4004 1] Year buttons "animations"
  (`SceneComponent.K2_SetRelativeLocation` (`self.Button_Plus`) (0.0 0.0 -1.0) false false)
  (`KismetSystemLibrary.Delay` 0.4)
  (`SceneComponent.K2_SetRelativeLocation` (`self.Button_Plus`) (0.0 0.0 0.0) false false)
  (if (< (`self.Year State`) 2)
    (set `self.Year State` (+ 1 (`self.Year State`)))
    (`self.Change Year State`)
    (`self.Change Year Layout`)
    (`self.Change Image On Widget`)
    (`self.Change Year On Widget`)))

(event `self.Button_Less.OnComponentBeginOverlap`
  (params (OverlappedComponent :type "PrimitiveComponent Object Reference") (OtherActor :type "Actor Object Reference") (OtherComp :type "PrimitiveComponent Object Reference") (OtherBodyIndex :type Integer) (bFromSweep :type Boolean) (SweepResult :type "HitResult Structure (by ref)"))
  ;[0.7801 0.4004 1] Year buttons "animations"
  (`SceneComponent.K2_SetRelativeLocation` (`self.Button_Less`) (0.0 0.0 -1.0) false false)
  (`KismetSystemLibrary.Delay` 0.4)
  (`SceneComponent.K2_SetRelativeLocation` (`self.Button_Less`) (0.0 0.0 0.0) false false)
  (if (> (`self.Year State`) 0)
    (set `self.Year State` (+ -1 (`self.Year State`)))
    (`self.Change Year State`)
    (`self.Change Year Layout`)
    (`self.Change Image On Widget`)
    (`self.Change Year On Widget`)))

(event `Change Year State`
  ;[1 0 0.2774] Updating year state on enum.
  (switch `int` (`self.Year State`)
    (:`Default`
      (set `self.Year State` 1))
    (:`0`
      (set `self.Year State Enum` "NewEnumerator0"))
    (:`1`
      (set `self.Year State Enum` "NewEnumerator1"))))

(event `Change Image On Widget`
  ;[1 0.8758 0.6159] Change the image directly into the widget
  (bind _aspanel_widget (cast `/Game/Widgets/Panel_Widget` (`WidgetComponent.GetUserWidgetObject` (`self.UI`))))
  (set `/Game/Widgets/Panel_Widget.Image Index` (`self.Year State`) _aspanel_widget)
  (`/Game/Widgets/Panel_Widget.Change Image On Widget` _aspanel_widget))

(event `Change Year On Widget`
  ;[1 0.1718 0.8634] Change the year text directly into the widget
  (bind _aspanel_widget (cast `/Game/Widgets/Panel_Widget` (`WidgetComponent.GetUserWidgetObject` (`self.UI`))))
  (set `/Game/Widgets/Panel_Widget.Year Index` (`self.Year State`) _aspanel_widget)
  (`/Game/Widgets/Panel_Widget.Change Year On Widget` _aspanel_widget))

(event `Change Year Layout`
  (switch `/Game/Blueprints/Enums/YearState_Enum` (`self.Year State Enum`)))

(fn `UserConstructionScript`)