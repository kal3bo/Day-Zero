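; Planet Blueprint that shows world population at different historical years as hologram points on the planet.
; The exposed ChangeTextureOnPlane event creates a dynamic instance of the hologram material on the PointsHologram component.
; It switches on the ChangeTexture year value to pick a matching points texture, from year 1 to 2020, and assigns it to the material's Points parameter.
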(event `Change Texture On Plane`
  ;[0 0 0] Exposed function to change the texture of the material on the particle FX in order to place less or more population on the planet
  (bind _returnvalue (`PrimitiveComponent.CreateDynamicMaterialInstance` (`self.Points_Hologram`) 0 "/Game/SciFiFX/Materials/M_Hologram_In.M_Hologram_In" "None"))
  (switch `/Game/Enums/TextureState_Enum` (`self.Change Texture`)
    (:`NewEnumerator0`
      (set `self.Points Texture` "/Game/SciFiFX/Textures/Points_Year_1.Points_Year_1"))
    (:`NewEnumerator1`
      (set `self.Points Texture` "/Game/SciFiFX/Textures/Points_Year_165.Points_Year_165"))
    (:`NewEnumerator2`
      (set `self.Points Texture` "/Game/SciFiFX/Textures/Points_Year_536.Points_Year_536"))
    (:`NewEnumerator3`
      (set `self.Points Texture` "/Game/SciFiFX/Textures/Points_Year_1030.Points_Year_1030"))
    (:`NewEnumerator4`
      (set `self.Points Texture` "/Game/SciFiFX/Textures/Points_Year_1501.Points_Year_1501"))
    (:`NewEnumerator5`
      (set `self.Points Texture` "/Game/SciFiFX/Textures/Points_Year_1796.Points_Year_1796"))
    (:`NewEnumerator6`
      (set `self.Points Texture` "/Game/SciFiFX/Textures/Points_Year_1880.Points_Year_1880"))
    (:`NewEnumerator7`
      (set `self.Points Texture` "/Game/SciFiFX/Textures/Points_Year_1960.Points_Year_1960"))
    (:`NewEnumerator8`
      (set `self.Points Texture` "/Game/SciFiFX/Textures/Points_Year_2020.Points_Year_2020")))
  (`MaterialInstanceDynamic.SetTextureParameterValue` _returnvalue "Points" (`self.Points Texture`)))

(fn `UserConstructionScript`)