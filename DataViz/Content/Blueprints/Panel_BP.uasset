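; Interactive in-world panel that shows an image, year, population and info text for one of nine selectable year states.
; Overlap components act as buttons with brief press animations: one toggles the panel's visibility, plus and minus step the clamped year index.
; Each change updates the enum, pushes the index into Panel_Widget, and fetches that year's text from Firebase via a VaRest GET request, displaying the raw response on arrival.
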(event `self.ReceiveBeginPlay`
  ;[0 0 0] Retreiving all the information when the level starts.
  (`self.Change Year State`)
  (`self.Change Year Layout`)
  (`self.Change Image On Widget`)
  (`self.Change Year On Widget`)
  (`self.Change Population On Widget`))

(event `self.Interactable.OnComponentBeginOverlap`
  (params (OverlappedComponent :type "PrimitiveComponent Object Reference") (OtherActor :type "Actor Object Reference") (OtherComp :type "PrimitiveComponent Object Reference") (OtherBodyIndex :type Integer) (bFromSweep :type Boolean) (SweepResult :type "HitResult Structure (by ref)"))
  (bind _plane (`self.Plane`))
  ;[1 0.2167 0.1869] Start button "animation"
  (`SceneComponent.SetHiddenInGame` (`self.Start_Button`) true false)
  (`KismetSystemLibrary.Delay` 0.4)
  (`SceneComponent.SetHiddenInGame` (`self.Start_Button`) false false)
  (if (`self.isWindowOn`)
    (`SceneComponent.SetHiddenInGame` _plane true false)
    (`SceneComponent.SetHiddenInGame` (`self.Lines`) true false)
    (`SceneComponent.SetHiddenInGame` (`self.UI`) true false)
    (set `self.isWindowOn` false)
    (else
      (`SceneComponent.SetHiddenInGame` _plane false false)
      (`SceneComponent.SetHiddenInGame` (`self.Lines`) false false)
      (`SceneComponent.SetHiddenInGame` (`self.UI`) false false)
      (set `self.isWindowOn` true))))

(event `self.Button_Plus.OnComponentBeginOverlap`
  (params (OverlappedComponent :type "PrimitiveComponent Object Reference") (OtherActor :type "Actor Object Reference") (OtherComp :type "PrimitiveComponent Object Reference") (OtherBodyIndex :type Integer) (bFromSweep :type Boolean) (SweepResult :type "HitResult Structure (by ref)"))
  ;[0.7801 0.4004 1] Year buttons "animations" & change the state of the year to display the correct information.
  (`SceneComponent.K2_SetRelativeLocation` (`self.Button_Plus`) (0.0 0.0 -1.0) false false)
  (`KismetSystemLibrary.Delay` 0.4)
  (`SceneComponent.K2_SetRelativeLocation` (`self.Button_Plus`) (0.0 0.0 0.0) false false)
  (if (< (`self.Year State`) 8)
    (set `self.Year State` (+ 1 (`self.Year State`)))
    (`self.Change Year State`)
    (`self.Change Year Layout`)
    (`self.Change Image On Widget`)
    (`self.Change Year On Widget`)
    (`self.Change Population On Widget`)))

(event `self.Button_Less.OnComponentBeginOverlap`
  (params (OverlappedComponent :type "PrimitiveComponent Object Reference") (OtherActor :type "Actor Object Reference") (OtherComp :type "PrimitiveComponent Object Reference") (OtherBodyIndex :type Integer) (bFromSweep :type Boolean) (SweepResult :type "HitResult Structure (by ref)"))
  ;[0.7801 0.4004 1] Year buttons "animations" & change the state of the year to display the correct information.
  (`SceneComponent.K2_SetRelativeLocation` (`self.Button_Less`) (0.0 0.0 -1.0) false false)
  (`KismetSystemLibrary.Delay` 0.4)
  (`SceneComponent.K2_SetRelativeLocation` (`self.Button_Less`) (0.0 0.0 0.0) false false)
  (if (> (`self.Year State`) 0)
    (set `self.Year State` (+ -1 (`self.Year State`)))
    (`self.Change Year State`)
    (`self.Change Year Layout`)
    (`self.Change Image On Widget`)
    (`self.Change Year On Widget`)
    (`self.Change Population On Widget`)))

(event `Change Year State`
  ;[1 0 0.2774] Updating year state on enum.
  (switch `int` (`self.Year State`)
    (:`Default`
      (set `self.Year State` 1))
    (:`0`
      (set `self.Year State Enum` "NewEnumerator0"))
    (:`1`
      (set `self.Year State Enum` "NewEnumerator1"))
    (:`2`
      (set `self.Year State Enum` "NewEnumerator2"))
    (:`3`
      (set `self.Year State Enum` "NewEnumerator3"))
    (:`4`
      (set `self.Year State Enum` "NewEnumerator4"))
    (:`5`
      (set `self.Year State Enum` "NewEnumerator5"))
    (:`6`
      (set `self.Year State Enum` "NewEnumerator6"))
    (:`7`
      (set `self.Year State Enum` "NewEnumerator7"))
    (:`8`
      (set `self.Year State Enum` "NewEnumerator8"))))

(event `Change Image On Widget`
  ;[1 0.8758 0.6159] Change the image directly into the widget
  (bind _aspanel_widget (cast `/Game/Widgets/Panel_Widget` (`WidgetComponent.GetUserWidgetObject` (`self.UI`))))
  (set `/Game/Widgets/Panel_Widget.Image Index` (`self.Year State`) _aspanel_widget)
  (`/Game/Widgets/Panel_Widget.Change Image On Widget` _aspanel_widget))

(event `Change Year On Widget`
  ;[1 0.1718 0.8634] Change the year text directly into the widget
  (bind _aspanel_widget (cast `/Game/Widgets/Panel_Widget` (`WidgetComponent.GetUserWidgetObject` (`self.UI`))))
  (set `/Game/Widgets/Panel_Widget.Year Index` (`self.Year State`) _aspanel_widget)
  (`/Game/Widgets/Panel_Widget.Change Year On Widget` _aspanel_widget))

(event `Change Population On Widget`
  (bind _aspanel_widget (cast `/Game/Widgets/Panel_Widget` (`WidgetComponent.GetUserWidgetObject` (`self.UI`))))
  (set `/Game/Widgets/Panel_Widget.Population Index` (`self.Year State`) _aspanel_widget)
  (`/Game/Widgets/Panel_Widget.Change Population On Widget` _aspanel_widget))

(event `Change Year Layout`
  ;[1 0 0.09028] HTTP request: access to the database information with the privided URL and changes the information text on UI.
  (`self.Make URL`)
  (`VaRestSubsystem.CallURL` (subsystem `VaRestSubsystem`) (`self.URL`) "GET" "binary" null (delegate `URL Response`)))

(event `URL Response`
  (params (Request :type "VaRestRequestJSON Object Reference"))
  ;[1 0 0.09028] HTTP request: access to the database information with the privided URL and changes the information text on UI.
  (bind _returnvalue (`VaRestRequestJSON.GetResponseContentAsString` Request true))
  (set `self.Information` _returnvalue)
  (bind _aspanel_widget (cast `/Game/Widgets/Panel_Widget` (`WidgetComponent.GetUserWidgetObject` (`self.UI`))))
  (set `/Game/Widgets/Panel_Widget.InfoText` (`KismetTextLibrary.Conv_StringToText` (`self.Information`)) _aspanel_widget)
  (`/Game/Widgets/Panel_Widget.Get_Information_Text_0` _aspanel_widget))

(event `Make URL`
  ;[1 0.8659 0.4917] Makes the URL combining the API address with the current Year State on Enum.
  (set `self.URL` (`KismetStringLibrary.Concat_StrStr` "https://from-day-zero.firebaseio.com/Years/" (`KismetSystemLibrary.MakeLiteralString` (`KismetSystemLibrary.MakeLiteralString` (`|GetEnumeratorNameAsString` (`self.Year State Enum`)))) ".json")))

(fn `UserConstructionScript`)